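; BP_BulletEnemy is an enemy projectile that damages the player character, BP_TPC_Platform, on overlap.
; Each tick it moves along its forward vector at its Speed, without sweeping.
; On overlapping the player character it spawns an explosion emitter and applies fixed damage, then destroys itself and prints a debug string.
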(event Collision|EventActorBeginOverlap
  (params (OtherActor :type Actor%20Object%20Reference))
  (bind _asbp_tpc_platform (Utilities|Casting|CastToBP_TPC_Platform OtherActor)
    (:then
      (Effects|SpawnEmitteratLocation "/Game/StarterContent/Particles/P_Explosion.P_Explosion" (Transformation|GetActorLocation))
      (Game|Damage|ApplyDamage _asbp_tpc_platform 1e+01 0 self))
    (:CastFailed
      _))
  (Actor|DestroyActor)
  (Development|PrintString "shoot"))

(event EventTick
  (params (DeltaSeconds :type Float%20%28single-precision%29))
  (Transformation|SetActorLocation (+ (Transformation|GetActorLocation) (* (* DeltaSeconds (Variables|Default|GetSpeed)) (Transformation|GetActorForwardVector))) false false))

(fn ConstructionScript)